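; Manager actor that drives ZED Manny avatars from Live Link animation subjects.
; On BeginPlay it connects to the first discovered message bus provider, and removes that source on EndPlay.
; Each Tick it diffs enabled animation subjects against an avatar map, spawning new avatars hidden and destroying missing ones.
; Existing avatars are made visible and receive height, floor-sticking and bone-scaling settings through their AnimBP, plus optional self-collision.
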(event `self.ReceiveEndPlay`
  (params (EndPlayReason :type "EEndPlayReason Enum" :default "Destroyed"))
  (`LiveLinkBlueprintLibrary.RemoveSource` (`self.Source Handle Ref`)))

(event `self.ReceiveBeginPlay`
  (bind _returnvalue (`LiveLinkMessageBusFinder.ConstructMessageBusFinder`))
  (bind _availableproviders (`LiveLinkMessageBusFinder.GetAvailableProviders` _returnvalue 0.2))
  (if (`KismetMathLibrary.Conv_IntToBool` (`KismetArrayLibrary.Array_Length` _availableproviders))
    (bind _sourcehandle (`LiveLinkMessageBusFinder.ConnectToProvider` (`|GetArrayItem` _availableproviders)))
    (bind _output_get (set `self.Source Handle Ref` _sourcehandle))
    (bind _returnvalue_2 (`LiveLinkBlueprintLibrary.GetSourceMachineName` _output_get))
    (`KismetSystemLibrary.PrintString` (`KismetStringLibrary.Concat_StrStr` "Connecting to " (`KismetTextLibrary.Conv_TextToString` _returnvalue_2)))
    (else
      (`KismetSystemLibrary.PrintString` "No Provinder Found!"))))

(event `self.ReceiveTick`
  (params (DeltaSeconds :type "Float (single-precision)"))
  (bind _value (`BlueprintMapLibrary.Map_Find` (`self.Avatars`) (`self.Current Subject`)))
  (bind _keys (`BlueprintMapLibrary.Map_Keys` (`self.Avatars`)))
  (set `self.remainingAvatars` _keys)
  (bind _returnvalue (`LiveLinkBlueprintLibrary.GetLiveLinkEnabledSubjectNames` false))
  (for _array_element _returnvalue
    (bind _output_get (set `self.Current Subject` _array_element))
    (bind _returnvalue_2 (`LiveLinkBlueprintLibrary.GetLiveLinkSubjectRole` _output_get)) ; Filter Animation Role only
    (if (== _returnvalue_2 "/Script/LiveLinkInterface.LiveLinkAnimationRole")
      (if (`BlueprintMapLibrary.Map_Contains` (`self.Avatars`) (`self.Current Subject`))
        (`KismetArrayLibrary.Array_RemoveItem` (`self.remainingAvatars`) (`self.Current Subject`)) ; Do nothing when existing ID.Only updates RemainingAvatar array
        (bind _asabp_zed_manny (cast `/Game/ZED/Blueprints/ABP_ZED_Manny` (`SkeletalMeshComponent.GetAnimInstance` (`self.GetComponentByClass` _value "/Script/Engine.SkeletalMeshComponent"))))
        (set `/Game/ZED/Blueprints/ABP_ZED_Manny.Height Offset` (`self.Height Offset`) _asabp_zed_manny)
        (set `/Game/ZED/Blueprints/ABP_ZED_Manny.Stick Avatar On Floor` (`self.Stick Avatar on Floor`) _asabp_zed_manny)
        (set `/Game/ZED/Blueprints/ABP_ZED_Manny.Bone Scaling` (`self.Bone Scaling - Experimental`) _asabp_zed_manny)
        (bind _asbp_zed_manny (cast `/Game/ZED/Blueprints/BP_ZED_Manny` _value))
        (`SceneComponent.SetVisibility` (`Actor.RootComponent` _asbp_zed_manny) true true)
        (if (`self.Enable Self Colision`)
          (`/Game/ZED/Blueprints/BP_ZED_Manny.Enable Self Collision` _asbp_zed_manny))
        (else
          (bind _returnvalue_3 (`|SpawnActorFromClass` "/Game/ZED/Blueprints/BP_ZED_Manny.BP_ZED_Manny_C" (`self.Init_pos`) "AlwaysSpawn" "OverrideRootScale" null null)) ; Add when New ID
          (`BlueprintMapLibrary.Map_Add` (`self.Avatars`) (`self.Current Subject`) _returnvalue_3)
          (bind _returnvalue_4 (`self.GetComponentByClass` _returnvalue_3 "/Script/Engine.SkeletalMeshComponent"))
          (bind _output_get_2 (set `self.Skeletal Mesh` _returnvalue_4))
          (`SceneComponent.SetVisibility` _output_get_2 false true)
          (bind _asabp_zed_manny_2 (cast `/Game/ZED/Blueprints/ABP_ZED_Manny` (`SkeletalMeshComponent.GetAnimInstance` _returnvalue_4))
            (:`then`
              (set `/Game/ZED/Blueprints/ABP_ZED_Manny.Live Link Subject` (`self.Current Subject`) _asabp_zed_manny_2)
              (set `/Game/ZED/Blueprints/ABP_ZED_Manny.Skeletal Mesh` (`self.Skeletal Mesh`) _asabp_zed_manny_2)
              (set `/Game/ZED/Blueprints/ABP_ZED_Manny.Height Offset` (`self.Height Offset`) _asabp_zed_manny_2)
              (set `/Game/ZED/Blueprints/ABP_ZED_Manny.Bone Scaling` (`self.Bone Scaling - Experimental`) _asabp_zed_manny_2)
              (set `/Game/ZED/Blueprints/ABP_ZED_Manny.Stick Avatar On Floor` (`self.Stick Avatar on Floor`) _asabp_zed_manny_2))
            (:`CastFailed`
              (`KismetSystemLibrary.PrintString` "Cast Failed")))))))
  ;[1 1 1] Destroy Avatars which are not longer detected in the scene
  (for _array_element_2 (`self.remainingAvatars`)
    (bind (_value_2 _returnvalue_5) (`BlueprintMapLibrary.Map_Find` (`self.Avatars`) _array_element_2))
    (if (== _returnvalue_5 true)
      (`self.K2_DestroyActor` _value_2)
      (`BlueprintMapLibrary.Map_Remove` (`self.Avatars`) _array_element_2) ; Remove no longer detected IDs
    )))

(fn `UserConstructionScript`)